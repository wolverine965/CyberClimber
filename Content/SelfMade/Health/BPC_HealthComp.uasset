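; Health component Blueprint that tracks an owner's hit points and signals death.
; CurrentHP starts at MaxHP on BeginPlay, and HandleDMG subtracts damage, clamping the result between zero and a hardcoded 100 rather than MaxHP.
; HandleDMG calls the OnDeath dispatcher whenever HP is at zero after a hit; the component's own bound handler only prints a debug "Death" message.
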(event Custom|HandleDMG
  (params (Damage :type Float%20%28double-precision%29))
  (Variables|Default|SetCurrentHP (Math|Float|Clamp(Float) (- (Variables|Default|GetCurrentHP) Damage) 0.0 1e+02))
  (if (<= (Variables|Default|GetCurrentHP) 0.0)
    (Default|CallOnDeath)))

(event Custom|CustomEvent
  (Development|PrintString "Death"))

(event EventBeginPlay
  (Variables|Default|SetCurrentHP (Variables|Default|GetMaxHP))
  (EventDispatchers|BindEventtoOnDeath (delegate Custom|CustomEvent)))

(event EventTick
  (params (DeltaSeconds :type Float%20%28single-precision%29)))