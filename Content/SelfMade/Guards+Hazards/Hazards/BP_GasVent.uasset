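; BP_GasVent is a hazard actor that slides along its mesh's forward vector from its placed location.
; BeginPlay computes the end point from MoveDistance and plays the PushPlayer timeline, scaled by MoveDuration, to lerp the actor's location without sweep.
; When the timeline finishes, it toggles ResettingLocation, which swaps the lerp endpoints, but nothing in the graph replays the timeline.
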(event EventBeginPlay
  (bind _returnvalue (Transformation|GetActorLocation))
  (Variables|Default|SetStaringLocation _returnvalue)
  (Variables|Default|SetEndingLocation (+ _returnvalue (* (Math|Vector|GetForwardVector (Variables|Default|GetStaticMesh)) (Variables|Default|GetMove%20Distance))))
  (Components|Timeline|SetPlayRate (Variables|Default|GetPushPlayer) (/ 1.0 (Variables|Default|GetMove%20Duration)))
  (bind _location (Timeline|PushPlayer PlayFromStart)
    (:Update
      (Transformation|SetActorLocation (Math|Vector|Lerp(Vector) (Math|Vector|SelectVector (Variables|Default|GetEndingLocation) (Variables|Default|GetStaringLocation) (Variables|Default|GetResettingLocation?)) (Math|Vector|SelectVector (Variables|Default|GetStaringLocation) (Variables|Default|GetEndingLocation) (Variables|Default|GetResettingLocation?)) _location) false false))
    (:Finished
      (if (Variables|Default|GetResettingLocation?)
        (Variables|Default|SetResettingLocation? false)
        (else
          (Variables|Default|SetResettingLocation? true))))))

(fn ConstructionScript)