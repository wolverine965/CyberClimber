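; Spline path mover that carries a referenced actor along its spline in a repeating cycle, filed under hazards.
; The construction script snaps that actor to the first spline point.
; On BeginPlay the timeline rate is set from TimelineLength, then its MovingPlatform track maps to distance along the spline to set world location each update without sweep.
; The timeline restarts from the start whenever it finishes.
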(event Custom|PlayTimeline
  (bind _spline (Variables|Default|GetSpline))
  (bind _movingplatform (Timeline|Timeline_0 PlayFromStart)
    (:Update
      (Transformation|SetActorLocation (Variables|Default|GetActor) (Spline|GetLocationatDistanceAlongSpline (Variables|Default|GetSpline) (Math|Float|Lerp 0.0 (Spline|GetDistanceAlongSplineatSplinePoint _spline (- (Spline|GetNumberOfSplinePoints _spline) 1)) _movingplatform) "World") false false))
    (:Finished
      (CallFunction|PlayTimeline))))

(event EventBeginPlay
  (Components|Timeline|SetPlayRate (Variables|Default|GetTimeline_0) (/ 1.0 (Variables|Default|GetTimelineLength)))
  (CallFunction|PlayTimeline))

(fn ConstructionScript
  (Transformation|SetActorLocation (Variables|Default|GetActor) (Spline|GetLocationatSplinePoint (Variables|Default|GetSpline) 0 "World") false false))