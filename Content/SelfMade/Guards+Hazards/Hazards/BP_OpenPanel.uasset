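; BP_OpenPanel is a hazard that damages BP_ThirdPersonCharacter actors touching its OpenPanel component.
; Entering the component's overlap applies BaseDmg once.
; Tick then polls the component's overlapping characters and applies BaseDmg to each valid one every frame, without delta-time scaling, so sustained damage depends on frame rate.
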(event OnComponentBeginOverlap(OpenPanel)
  (params (OverlappedComponent :type Primitive%20Component%20Object%20Reference) (OtherActor :type Actor%20Object%20Reference) (OtherComp :type Primitive%20Component%20Object%20Reference) (OtherBodyIndex :type Integer) (bFromSweep :type Boolean) (SweepResult :type Hit%20Result%20Structure%20%28by%20ref%29))
  (bind _asbp_third_person_character (Utilities|Casting|CastToBP_ThirdPersonCharacter OtherActor))
  (Game|Damage|ApplyDamage _asbp_third_person_character (Variables|Default|GetBaseDmg) 0 0))

(event EventBeginPlay)

(event EventTick
  (params (DeltaSeconds :type Float%20%28single-precision%29))
  (bind _openpanel (Variables|Default|GetOpenPanel))
  (bind _overlappingactors (Collision|GetOverlappingActors _openpanel "/Game/ThirdPerson/Blueprints/BP_ThirdPersonCharacter.BP_ThirdPersonCharacter_C" :!class /Script/Engine.PrimitiveComponent))
  (if (Utilities|Array|IsNotEmpty _overlappingactors)
    (for _array_element _overlappingactors
      (Utilities|IsValid _array_element
        (:Is%20Valid
          (Game|Damage|ApplyDamage _array_element (Variables|Default|GetBaseDmg) 0 0))))))

(fn ConstructionScript)