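; Hazard-folder Blueprint meant to move an array of actors along a spline in a repeating loop.
; A self-restarting Timeline, rate-scaled by TimelineLength, feeds a Lerp plus per-index spacing, wrapping distances past the spline's end.
; The Lerp's endpoints are both zero here, so only the spacing affects position.
; The Construction Script also places the actors on the spline, leaving its spacing calculation unused.
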(event Custom|PlayTimeline
  (bind _spline (Variables|Default|GetSpline))
  (bind _returnvalue (Spline|GetSplineLength _spline))
  (bind _movingplatform (Timeline|Timeline_0 PlayFromStart)
    (:Update
      (for (_array_element _array_index) (Variables|Default|GetActor)
        (bind _output_get (Variables|Default|SetDistanceAlongSpline (+ (Math|Float|Lerp 0.0 0.0 _movingplatform) (* _array_index (Variables|Default|GetOffestBetweenActor)))))
        (if (> _output_get _returnvalue)
          (Variables|Default|SetDistanceAlongSpline (- (Variables|Default|GetDistanceAlongSpline) _returnvalue)))
        (Transformation|SetActorLocationAndRotation _array_element (Spline|GetLocationatDistanceAlongSpline (Variables|Default|GetSpline) (Variables|Default|GetDistanceAlongSpline) "World"))))
    (:Finished
      (CallFunction|PlayTimeline))))

(event EventBeginPlay
  (Components|Timeline|SetPlayRate (Variables|Default|GetTimeline_0) (/ 1.0 (Variables|Default|GetTimelineLength)))
  (CallFunction|PlayTimeline))

(fn ConstructionScript
  (for (_array_element _array_index) (Variables|Default|GetActor)
    (Transformation|SetActorLocationAndRotation _array_element (Spline|GetLocationatDistanceAlongSpline (Variables|Default|GetSpline) (Variables|Default|GetDistanceAlongSpline) "World"))))