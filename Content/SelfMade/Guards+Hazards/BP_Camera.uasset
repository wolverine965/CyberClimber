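; Security camera hazard that sweeps back and forth and alerts guards when its detection box is overlapped.
; A ping-pong timeline lerps camera yaw, while a per-tick trace from the scene capture positions a status LED decal at the impact point.
; On overlap, it flags detection in the game instance, switches the decal material, stops the sweep, and sends the player pawn to sphere-overlapped guards confirmed by line traces.
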(event OnComponentBeginOverlap(Box)
  (params (OverlappedComponent :type Primitive%20Component%20Object%20Reference) (OtherActor :type Actor%20Object%20Reference) (OtherComp :type Primitive%20Component%20Object%20Reference) (OtherBodyIndex :type Integer) (bFromSweep :type Boolean) (SweepResult :type Hit%20Result%20Structure%20%28by%20ref%29))
  ;[0.15 0.15 0.15 0.5] Alert Guards Logic
  (Variables|/Game/SelfMade/GameInstance/BP_GameInstance.BP_GameInstance_C|SetIsPlayerDetected? (Variables|Default|GetGameInstance) true)
  (Rendering|Components|Decal|SetDecalMaterial (Variables|Default|GetStatusLED) "/Game/SelfMade/Guards+Hazards/Materials/M_Camera_Found.M_Camera_Found")
  (CallFunction|BlockTimeline)
  (bind _outactors (Collision|SphereOverlapActors "0, 0, 0" 3e+03 (Utilities|Array|MakeArray "ObjectTypeQuery3") "/Game/SelfMade/Guards+Hazards/BP_Guard.BP_Guard_C"))
  (for _array_element _outactors
    (bind _asbp_guard (Utilities|Casting|CastToBP_Guard _array_element))
    (bind (_outhit _returnvalue) (Collision|LineTraceByChannel (Transformation|GetActorLocation self) (Transformation|GetActorLocation _asbp_guard) "TraceTypeQuery1" false 0 "Persistent" true "(R=1.000000,G=0.000000,B=0.000000,A=1.000000)" "(R=0.000000,G=1.000000,B=0.000000,A=1.000000)" 2.5))
    (if _returnvalue
      (bind _asbp_guard_2 (Utilities|Casting|CastToBP_Guard (.HitActor (Collision|BreakHitResult _outhit)))
        (:then
          (if true
            (Class|BPIGuardAlert|ReceiveAlert(Message) _asbp_guard_2 (Game|Player|GetPlayerPawn 0))))
        (:CastFailed
          (Development|PrintString "Missed Call"))))))

(event Custom|Block%20Timeline
  (bind _camera (Variables|Default|GetCamera))
  (bind _relativerotation (Variables|/Script/Engine.SceneComponent|GetRelativeRotation _camera))
  ;[0.15 0.15 0.15 0.5] Camera Move Logic
  (bind _moving_value (Timeline|Camera%20Move Stop)
    (:Update
      (Transformation|SetRelativeRotation (Variables|Default|GetCamera) (Math|Rotator|Lerp(Rotator) (Math|Rotator|MakeRotator (.roll _relativerotation) (.pitch _relativerotation) -45.0) (Math|Rotator|MakeRotator (.roll _relativerotation) (.pitch _relativerotation) 45.0) _moving_value) false false))
    (:Finished
      (if (Variables|Default|GetIsRestart?)
        (Variables|Default|SetIsRestart? false)
        (Timeline|Camera%20Move Play)
        (else
          (Variables|Default|SetIsRestart? true)
          (Timeline|Camera%20Move Reverse))))))

(event EventBeginPlay
  (bind _camera (Variables|Default|GetCamera))
  (bind _relativerotation (Variables|/Script/Engine.SceneComponent|GetRelativeRotation _camera))
  ;[0.15 0.15 0.15 0.5] Camera Move Logic
  (bind _asbp_game_instance (Utilities|Casting|CastToBP_GameInstance (Game|GetGameInstance)))
  (Variables|Default|SetGameInstance _asbp_game_instance)
  (bind _moving_value (Timeline|Camera%20Move Play)
    (:Update
      (Transformation|SetRelativeRotation (Variables|Default|GetCamera) (Math|Rotator|Lerp(Rotator) (Math|Rotator|MakeRotator (.roll _relativerotation) (.pitch _relativerotation) -45.0) (Math|Rotator|MakeRotator (.roll _relativerotation) (.pitch _relativerotation) 45.0) _moving_value) false false))
    (:Finished
      (if (Variables|Default|GetIsRestart?)
        (Variables|Default|SetIsRestart? false)
        (Timeline|Camera%20Move Play)
        (else
          (Variables|Default|SetIsRestart? true)
          (Timeline|Camera%20Move Reverse))))))

(event EventTick
  (params (DeltaSeconds :type Float%20%28single-precision%29))
  ;[0.15 0.15 0.15 0.5] pawn detection
  (bind _outhit (Collision|LineTraceByChannel (Transformation|GetWorldLocation (Variables|Default|GetSceneCaptureComponent2D)) (* (Math|Vector|GetForwardVector (Variables|Default|GetSceneCaptureComponent2D)) 6e+02) "TraceTypeQuery1" false 0 "ForOneFrame"))
  (Transformation|SetWorldLocationAndRotation (Variables|Default|GetStatusLED) (.ImpactPoint (Collision|BreakHitResult _outhit)) (Math|Conversions|RotationFromXVector (.ImpactNormal (Collision|BreakHitResult _outhit))) false false))

(fn ConstructionScript)