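; BP_Punk is a melee enemy character that wanders random navigable points and can chase and punch pawns it sees.
; PawnSensing starts a detection message on the seen pawn, cleared after a second without sightings, and drives pursuit when ShouldChase is set.
; Reaching the target plays a punch montage, with a timer-triggered arm-socket sphere trace to apply damage.
; Incoming damage feeds a health component, whose death event ragdolls the mesh.
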(event OnDeath(BPC_HealthComp)
  (bind _mesh (Variables|Character|GetMesh))
  ;[0.15 0.15 0.15 0.5] Full Damage Logic
  (Collision|SetCollisionEnabled (Variables|Collision|GetCapsuleComponent) "PhysicsOnly")
  (Collision|SetCollisionProfileName _mesh "Ragdoll" true :!class /Script/Engine.PrimitiveComponent)
  (Physics|SetSimulatePhysics _mesh true)
  (Collision|SetCollisionEnabled _mesh "PhysicsOnly"))

(event OnSeePawn(PawnSensing)
  (params (Pawn :type Pawn%20Object%20Reference))
  (bind _self self)
  (Utilities|FlowControl|Sequence
    (:then_0
      (Utilities|FlowControl|Sequence
        (:then_0
          (Utilities|FlowControl|DoOnce false :!label _label
            (:Completed
              (Class|BPDetectionInterface|StartDetection(Message) Pawn _self))))
        (:then_1
          (if (Variables|Default|GetShouldChase?)
            (AI|AIMoveTo _self "0, 0, 0" Pawn 75.0 false
              (:OnSuccess
                (CallFunction|StartFight)))))))
    (:then_1
      (Utilities|FlowControl|RetriggerableDelay 1.0)
      (Class|BPDetectionInterface|StopDetection(Message) Pawn)
      (goto _label Reset))))

(event Custom|Punch%20Trace
  (bind _mesh (Variables|Character|GetMesh))
  (bind (_outhit _returnvalue) (Collision|SphereTraceForObjects (.location (Transformation|GetSocketTransform _mesh "UpperArm_Trace" "RTS_World")) (.location (Transformation|GetSocketTransform _mesh "Hand_Trace" "RTS_World")) 25.0 (Utilities|Array|MakeArray "ObjectTypeQuery3") false 0 "ForDuration" true "(R=1.000000,G=0.000000,B=0.000000,A=1.000000)" "(R=0.000000,G=1.000000,B=0.000000,A=1.000000)" 0.1))
  (if _returnvalue
    (Game|Damage|ApplyDamage (.HitActor (Collision|BreakHitResult _outhit)) 1e+01 0 0)))

(event Custom|MoveToRandomLocation
  (bind _randomlocation (Class|NavigationSystemV1|GetRandomLocationinNavigableRadius (Transformation|GetActorLocation) 1e+03 0 0))
  (AI|AIMoveTo self _randomlocation 0 7e+01 false
    (:OnSuccess
      (CallFunction|MovetoRandomLocation))))

(event Custom|StartFight
  (if (Variables|Default|GetCanAttack?)
    (Variables|Default|SetCanAttack? false)
    (bind _returnvalue (Animation|PlayAnimMontage "/Game/Characters/Mannequins/Anims/Unarmed/Attack/MN_FALCONPUNCH.MN_FALCONPUNCH" 1.0 "None"))
    (Development|PrintString (Utilities|String|ToString(Float) _returnvalue))
    (Utilities|FlowControl|RetriggerableDelay _returnvalue)
    (Variables|Default|SetCanAttack? true)))

(event EventStartChase
  (Variables|Default|SetShouldChase? true))

(event EventStopChase
  (bind _self self)
  (Variables|Default|SetShouldChase? false)
  (AI|AIMoveTo _self "0, 0, 0" _self 7e+01 false))

(event EventBeginPlay
  (Collision|SetCollisionResponsetoChannel (Variables|Character|GetMesh) "ECC_Camera" "ECR_Ignore")
  (CallFunction|MovetoRandomLocation))

(event Game|Damage|EventAnyDamage
  (params (Damage :type Float%20%28single-precision%29) (DamageType :type Damage%20Type%20Object%20Reference) (InstigatedBy :type Controller%20Object%20Reference) (DamageCauser :type Actor%20Object%20Reference))
  (bind _bpc_healthcomp (Variables|Default|GetBPC_HealthComp))
  ;[0.15 0.15 0.15 0.5] Full Damage Logic
  ;;[0.15 0.15 0.15 0.5] Damage Logic
  (if (not (Variables|/Game/SelfMade/Health/BPC_HealthComp.BPC_HealthComp_C|GetbIsDeath (Variables|Default|GetBPC_HealthComp)))
    (Default|HandleDMG _bpc_healthcomp Damage)
    (Development|PrintString (Utilities|String|Append "Current Health:" (Utilities|String|ToString(Float) (Variables|/Game/SelfMade/Health/BPC_HealthComp.BPC_HealthComp_C|GetCurrentHP _bpc_healthcomp))) true true "(R=1.000000,G=0.000000,B=0.000000,A=1.000000)")))

(event EventStartPunchTrace
  (bind _returnvalue (Utilities|Time|SetTimerbyEvent (delegate Custom|Punch%20Trace) 0.1))
  (Variables|Default|SetPunchTraceLoop _returnvalue))

(event EventStopPunchTrace
  (bind _punchtraceloop (Variables|Default|GetPunchTraceLoop))
  (if (Utilities|Time|IsValidTimerHandle _punchtraceloop)
    (Utilities|Time|ClearandInvalidateTimerbyHandle _punchtraceloop)))

(fn ConstructionScript)