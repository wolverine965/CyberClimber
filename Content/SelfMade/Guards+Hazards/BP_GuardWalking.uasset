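; BP_GuardWalking is a patrolling guard that can spot, chase and damage the player.
; It loops through waypoints with AI MoveTo, pausing briefly at each, and resumes patrol when a chase stops.
; Pawn sensing toggles the seen pawn's detection message through a DoOnce and retriggerable delay, and triggers pursuit and an alert when chasing is enabled.
; An Alert event sends it toward the player, and capsule hits on the player character apply damage.
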(event OnSeePawn(PawnSensing)
  (params (Pawn :type Pawn%20Object%20Reference))
  (bind _self self)
  (Utilities|FlowControl|Sequence
    (:then_0
      (Utilities|FlowControl|Sequence
        (:then_0
          (Utilities|FlowControl|DoOnce false :!label _label
            (:Completed
              (Class|BPDetectionInterface|StartDetection(Message) Pawn _self))))
        (:then_1
          (if (Variables|Default|GetShouldChase?)
            (CallFunction|ReceiveAlert (Game|Player|GetPlayerPawn 0))
            (AI|AIMoveTo _self "0, 0, 0" Pawn 5.0 false)))))
    (:then_1
      (Utilities|FlowControl|RetriggerableDelay 0.5)
      (Class|BPDetectionInterface|StopDetection(Message) Pawn)
      (goto _label Reset))))

(event OnComponentHit(CapsuleComponent)
  (params (HitComponent :type Primitive%20Component%20Object%20Reference) (OtherActor :type Actor%20Object%20Reference) (OtherComp :type Primitive%20Component%20Object%20Reference) (NormalImpulse :type Vector :default "0, 0, 0") (Hit :type Hit%20Result%20Structure%20%28by%20ref%29))
  (bind _asbp_third_person_character (Utilities|Casting|CastToBP_ThirdPersonCharacter OtherActor))
  (Development|PrintString "Hit")
  (Game|Damage|ApplyDamage _asbp_third_person_character 25.0 0 0 "/Script/Engine.DamageType"))

(event Custom|Follow%20Waypoints
  (AI|AIMoveTo self "0, 0, 0" (Utilities|Array|Get(acopy) (Variables|Default|GetWayPoint) (Variables|Default|GetCurrentWayPoint)) 5.0 false
    (:OnSuccess
      (Math|Integer|IncrementInt (Variables|Default|GetCurrentWayPoint)
        (:%20%20
          (if (>= (Variables|Default|GetCurrentWayPoint) (Utilities|Array|Length (Variables|Default|GetWayPoint)))
            (Variables|Default|SetCurrentWayPoint 0))
          (Utilities|FlowControl|Delay 2.0)
          (CallFunction|FollowWaypoints))))
    (:OnFail
      (Development|PrintString "Oops"))))

(event EventAlert
  (params (PlayerRef :type Actor%20Object%20Reference))
  (AI|AIMoveTo self "0, 0, 0" PlayerRef 5.0 false))

(event EventStartChase
  (Variables|Default|SetShouldChase? true))

(event EventStopChase
  (Variables|Default|SetShouldChase? false)
  ;[0.15 0.15 0.15 0.5] They have to go back to patrol or default location
  (CallFunction|FollowWaypoints))

(event EventBeginPlay
  (CallFunction|FollowWaypoints))

(fn ConstructionScript)